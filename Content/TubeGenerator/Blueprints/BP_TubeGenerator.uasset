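; BP_TubeGenerator is an actor that procedurally assembles a chain of tube meshes in its Construction Script.
; An Evolution-driven loop adds static mesh components, each randomly picked from the SMTubeList map by integer key.
; Each mesh's Input_0 socket location is added, unrotated, to the next position, while its rotation replaces the stored one.
; Only that rotation's yaw is reused, feeding the next piece's roll.
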(fn `UserConstructionScript`
  (bind (_rotation_roll _rotation_pitch _rotation_yaw) (`KismetMathLibrary.BreakRotator` (`self.Rotation`)))
  (bind _sm_tubelist (`self.SM_TubeList`))
  (for _ (range (+ (`self.Evolution`) 1))
    (bind _returnvalue (`AddComponent|NODE_AddStaticMeshComponent-3` :`RelativeTransform` (`KismetMathLibrary.MakeTransform` (`self.New_Pos`) (`KismetMathLibrary.MakeRotator` _rotation_yaw))))
    (`StaticMeshComponent.SetStaticMesh` _returnvalue (`BlueprintMapLibrary.Map_Find` _sm_tubelist (`KismetMathLibrary.RandomIntegerInRange` 1 (`BlueprintMapLibrary.Map_Length` _sm_tubelist))))
    (bind _returnvalue_2 (`StaticMesh.FindSocket` (`StaticMeshComponent.StaticMesh` _returnvalue) "Input_0"))
    (set `self.New_Pos` (+ (`StaticMeshSocket.RelativeLocation` _returnvalue_2) (`self.New_Pos`)))
    (set `self.Rotation` (`StaticMeshSocket.RelativeRotation` _returnvalue_2))))